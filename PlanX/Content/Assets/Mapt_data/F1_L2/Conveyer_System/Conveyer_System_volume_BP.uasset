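; Conveyor belt volume Blueprint that carries any actor overlapping it along the actor's forward direction.
; Each Tick it gets the actors overlapping Volume and offsets their root components by forward vector, SpeedOfConveyer and delta time, without sweeping for collision.
; The construction script applies the inverse of the actor's scale to DirectionPointer, so the pointer keeps its size when the volume is scaled.
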(event EventBeginPlay)

(event Collision|EventActorBeginOverlap
  (params (OtherActor :type Actor%20Object%20Reference)))

(event EventTick
  (params (DeltaSeconds :type Float%20%28single-precision%29))
  (for _array_element (Collision|GetOverlappingActors (Variables|Default|Getvolume) 0 :!class /Script/Engine.PrimitiveComponent)
    (Transformation|AddWorldOffset (Variables|/Script/Engine.Actor|GetRootComponent _array_element) (* (Math|Vector|GetForwardVector (Transformation|GetActorRotation)) (* DeltaSeconds (Variables|Default|GetSpeed_of_Conveyer))) false false)))

(fn ConstructionScript
  (Transformation|SetRelativeScale3D (Variables|Default|Getdirection_pointer) (/ "1.000000,1.000000,1.000000" (Transformation|GetActorScale3D))))