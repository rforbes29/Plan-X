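; Level-design strip generator Blueprint that lays a chosen static mesh along an editable spline.
; The construction script adds one spline mesh component per spline point, sets its mesh and forward axis, attaches it to the spline and enables query-only collision.
; Segments take local location and tangent from the spline, but the next point's tangent and location feed EndPos and EndTangent swapped, and the loop includes the last point.
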(event EventBeginPlay)

(event Collision|EventActorBeginOverlap
  (params (OtherActor :type Actor%20Object%20Reference)))

(event EventTick
  (params (DeltaSeconds :type Float%20%28single-precision%29)))

(fn ConstructionScript
  (for _index (range 0 (- (Spline|GetNumberOfSplinePoints (Variables|Default|GetSpline)) 1))
    (bind _returnvalue (AddComponent|AddSplineMeshComponent false))
    (Variables|Default|Settarget _returnvalue)
    (Utilities|FlowControl|Sequence
      (:then_0
        (Components|StaticMesh|SetStaticMesh (Variables|Default|Gettarget) (Variables|Default|GetStatic%20Mesh)))
      (:then_1
        (SplineMesh|SetForwardAxis (Variables|Default|Gettarget) (Variables|Default|GetForward%20axis) true))
      (:then_2
        (Transformation|AttachComponentToComponent (Variables|Default|Gettarget) (Variables|Default|GetSpline) "None" "KeepRelative" "KeepRelative" "KeepRelative" true))
      (:then_3
        (Collision|SetCollisionEnabled (Variables|Default|Gettarget) "QueryOnly"))
      (:then_4
        (SplineMesh|SetStartandEnd (Variables|Default|Gettarget) (Spline|GetLocationatSplinePoint (Variables|Default|GetSpline) _index "Local") (Spline|GetTangentatSplinePoint (Variables|Default|GetSpline) _index "Local") (Spline|GetTangentatSplinePoint (Variables|Default|GetSpline) (+ _index 1) "Local") (Spline|GetLocationatSplinePoint (Variables|Default|GetSpline) (+ _index 1) "Local") true :!class /Script/Engine.SplineMeshComponent)))))