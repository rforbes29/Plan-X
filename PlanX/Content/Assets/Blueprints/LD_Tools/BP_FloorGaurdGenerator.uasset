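; Level design tool that generates a floor guard strip along an editable spline in the construction script.
; It syncs a per-point data array to the spline, then BuildStripElement adds spline meshes per segment, blending roll, width and thickness, with optional looping and query collision.
; Per-point flags add left/right light prop meshes, though a note marks this as broken.
; An optional debug pass labels each point with its index.
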(event EventBeginPlay)

(event Collision|EventActorBeginOverlap
  (params (OtherActor :type Actor%20Object%20Reference)))

(event EventTick
  (params (DeltaSeconds :type Float%20%28single-precision%29)))

(fn ConstructionScript
  (bind _stipdataarray (Variables|StripSetup|GetStipDataArray))
  (Utilities|FlowControl|Sequence
    (:then_0
      ;[0.3517 1 0.4997] Get and set the number of spline points
      (Variables|SplinePointandindexvalues|SetNumOfSplinePoints (Spline|GetNumberOfSplinePoints (Variables|Default|GetSpline))))
    (:then_1
      ;[0.42 1 0.3989] Comment
      (Math|Integer|CompareInt (Utilities|Array|Length (Variables|StripSetup|GetStipDataArray)) (Variables|SplinePointandindexvalues|GetNumOfSplinePoints) :!label _label
        (:>
          (Utilities|Array|RemoveIndex _stipdataarray (Utilities|Array|LastIndex _stipdataarray))
          (goto _label))
        (:<
          (Utilities|Array|Add (Variables|StripSetup|GetStipDataArray) (Variables|SplinePointandindexvalues|GetStripMeshDefaults))
          (goto _label))))
    (:then_2
      (for _index (range 0 (- (Variables|SplinePointandindexvalues|GetNumOfSplinePoints) (Math|Integer|SelectInt 1 2 (Variables|StripSetup|GetLooping%20strip%20bool))))
        (Variables|SplinePointandindexvalues|SetCurrent%20Loop%20Index _index)
        (Variables|StripSetup|SetDraw%20Left%20Light%20Prop (.leftlightprop (Utilities|Array|Get(acopy) (Variables|StripSetup|GetStipDataArray) (Variables|SplinePointandindexvalues|GetCurrent%20Loop%20Index))))
        (Variables|StripSetup|SetDraw%20Right%20Light%20Prop (.rightlightprop (Utilities|Array|Get(acopy) (Variables|StripSetup|GetStipDataArray) (Variables|SplinePointandindexvalues|GetCurrent%20Loop%20Index))))
        (Utilities|FlowControl|Sequence
          (:then_0
            ;[0.345 1 0.2628] Builds Strip element
            (CallFunction|BuildStripElement (Variables|SplinePointandindexvalues|GetCurrent%20Loop%20Index) (Variables|StaticMeshes|GetStripMesh)))
          (:then_1
            ;[0 0 0] Dosn't work, don't intend to fix any time soon. The idea is that when true, a point light is spawned next to the spline (current spline).
            (if (Variables|StripSetup|GetDraw%20Left%20Light%20Prop)
              (CallFunction|BuildStripElement (Variables|SplinePointandindexvalues|GetCurrent%20Loop%20Index) (Variables|StaticMeshes|GetLeft%20Light%20Prop))))
          (:then_2
            (if (Variables|StripSetup|GetDraw%20Right%20Light%20Prop)
              (CallFunction|BuildStripElement (Variables|SplinePointandindexvalues|GetCurrent%20Loop%20Index) (Variables|StaticMeshes|GetRight%20Light%20Prop)))))))
    (:then_3
      ;[0.1332 1 0.1727] as bool-Addes the current index to the location at the spline point
      (if (Variables|StripSetup|GetDraw%20Stip%20Num)
        (for _index_2 (range 0 (- (Variables|SplinePointandindexvalues|GetNumOfSplinePoints) 1))
          (Variables|SplinePointandindexvalues|SetCurrent%20Stip%20Point (Utilities|String|ToString(Integer) _index_2))
          (bind _returnvalue (AddComponent|AddTextRenderComponent false (Math|Transform|MakeTransform (Math|Vector|MakeVector (.X (Math|Vector|BreakVector (.Location (Spline|GetLocationandTangentatSplinePoint (Variables|Default|GetSpline) _index_2 "Local")))) (.Y (Math|Vector|BreakVector (.Location (Spline|GetLocationandTangentatSplinePoint (Variables|Default|GetSpline) _index_2 "Local")))) (+ (.Z (Math|Vector|BreakVector (.Location (Spline|GetLocationandTangentatSplinePoint (Variables|Default|GetSpline) _index_2 "Local")))) 2e+01)) (Math|Conversions|RotationFromXVector (* (.Tangent (Spline|GetLocationandTangentatSplinePoint (Variables|Default|GetSpline) _index_2 "Local")) -1.0)))))
          (Rendering|Components|TextRender|SetText _returnvalue (Utilities|Text|ToText(String) (Variables|SplinePointandindexvalues|GetCurrent%20Stip%20Point))))))))

(fn BuildStripElement
  (params (CurrentLoopIndex :type Integer) (StripElementMesh :type Static%20Mesh%20Object%20Reference))
  (LocalVariables|SetPrivate_CurrentLoopIndex CurrentLoopIndex)
  (LocalVariables|SetPrivate_NextLoopIndex (Math|Integer|%(Integer) (+ CurrentLoopIndex 1) (Variables|SplinePointandindexvalues|GetNumOfSplinePoints)))
  (LocalVariables|SetPrivate_StripElementMesh StripElementMesh)
  (Utilities|FlowControl|Sequence
    (:then_0
      (LocalVariables|SetPrivate_StartLocation (.Location (Spline|GetLocationandTangentatSplinePoint (Variables|Default|GetSpline) (LocalVariables|GetPrivate_CurrentLoopIndex) "Local")))
      (LocalVariables|SetPrivate_StartTangent (.Tangent (Spline|GetLocationandTangentatSplinePoint (Variables|Default|GetSpline) (LocalVariables|GetPrivate_CurrentLoopIndex) "Local")))
      (LocalVariables|SetPrivate_EndLocation (.Location (Spline|GetLocationandTangentatSplinePoint (Variables|Default|GetSpline) (LocalVariables|GetPrivate_NextLoopIndex) "Local")))
      (LocalVariables|SetPrivate_EndTangent (.Tangent (Spline|GetLocationandTangentatSplinePoint (Variables|Default|GetSpline) (LocalVariables|GetPrivate_NextLoopIndex) "Local")))
      (LocalVariables|SetPrivate_StartRoll (.banklightstipamount (Utilities|Array|Get(acopy) (Variables|StripSetup|GetStipDataArray) (LocalVariables|GetPrivate_CurrentLoopIndex))))
      (LocalVariables|SetPrivate_StartScale (Math|Vector2D|MakeVector2D (.lightstipwidth (Utilities|Array|Get(acopy) (Variables|StripSetup|GetStipDataArray) (LocalVariables|GetPrivate_CurrentLoopIndex))) (.lightstipthickness (Utilities|Array|Get(acopy) (Variables|StripSetup|GetStipDataArray) (LocalVariables|GetPrivate_CurrentLoopIndex)))))
      (LocalVariables|SetPrivate_EndRoll (.banklightstipamount (Utilities|Array|Get(acopy) (Variables|StripSetup|GetStipDataArray) (LocalVariables|GetPrivate_NextLoopIndex))))
      (LocalVariables|SetPrivate_EndScale (Math|Vector2D|MakeVector2D (.lightstipwidth (Utilities|Array|Get(acopy) (Variables|StripSetup|GetStipDataArray) (LocalVariables|GetPrivate_NextLoopIndex))) (.lightstipthickness (Utilities|Array|Get(acopy) (Variables|StripSetup|GetStipDataArray) (LocalVariables|GetPrivate_NextLoopIndex))))))
    (:then_1
      (bind _returnvalue (AddComponent|AddSplineMeshComponent false))
      (LocalVariables|SetPrivate_CurrentSplineMesh _returnvalue)
      (Components|StaticMesh|SetStaticMesh (LocalVariables|GetPrivate_CurrentSplineMesh) (LocalVariables|GetPrivate_StripElementMesh))
      (SplineMesh|SetStartandEnd (LocalVariables|GetPrivate_CurrentSplineMesh) (LocalVariables|GetPrivate_StartLocation) (LocalVariables|GetPrivate_StartTangent) (LocalVariables|GetPrivate_EndLocation) (LocalVariables|GetPrivate_EndTangent) true :!class /Script/Engine.SplineMeshComponent)
      (Class|SplineMeshComponent|SetStartRoll (LocalVariables|GetPrivate_CurrentSplineMesh) (LocalVariables|GetPrivate_StartRoll) true)
      (Class|SplineMeshComponent|SetEndRoll (LocalVariables|GetPrivate_CurrentSplineMesh) (LocalVariables|GetPrivate_EndRoll) true)
      (SplineMesh|SetStartScale (LocalVariables|GetPrivate_CurrentSplineMesh) (LocalVariables|GetPrivate_StartScale) true :!class /Script/Engine.SplineMeshComponent)
      (SplineMesh|SetEndScale (LocalVariables|GetPrivate_CurrentSplineMesh) (LocalVariables|GetPrivate_EndScale) true :!class /Script/Engine.SplineMeshComponent)
      (Collision|SetCollisionEnabled (LocalVariables|GetPrivate_CurrentSplineMesh) (select (Variables|StripSetup|GetcollisonToggle) "QueryOnly" "NoCollision")))))